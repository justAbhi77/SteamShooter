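; Blueprint for the Blaster player character that handles the overhead player name and the sniper scope overlay.
; On BeginPlay it writes the PlayerState name to the overhead widget, and non-authority instances also pass it to ServerSetPlayerName.
; The scope event lazily creates and reuses one scope widget, playing its zoom animation forward or reversed with matching sounds.
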(event Custom|Server_SetPlayerName
  (params (Name :type String))
  (CallFunction|FSetNameonWidget Name))

(event EventShowSniperScopeWidget
  (params (bShowScope :type Boolean))
  (Utilities|FlowControl|Sequence
    (:then_0
      (Variables|Default|GetSniperScopeWidget
        (:then)
        (:else
          (bind _returnvalue (UserInterface|CreateWidget "/Game/Blueprints/Hud/WBP_SniperScope.WBP_SniperScope_C"))
          (bind _output_get (Variables|Default|SetSniperScopeWidget _returnvalue))
          (UserInterface|Viewport|AddtoViewport _output_get 0))))
    (:then_1
      (Variables|Default|GetSniperScopeWidget
        (:then
          (if bShowScope
            (UserInterface|Animation|PlayAnimation (Variables|Default|GetSniperScopeWidget) (Variables|/Game/Blueprints/Hud/WBP_SniperScope.WBP_SniperScope_C|GetScopeZoomIn (Variables|Default|GetSniperScopeWidget)) 0.0 1 "Forward" 1.0 false)
            (Audio|PlaySound2D "/Game/Assets/MilitaryWeapSilver/Sound/SniperRifle/Cues/SniperRifle_ZoomIn_Cue.SniperRifle_ZoomIn_Cue" 1.0 1.0 0.0 0 0)
            (else
              (UserInterface|Animation|PlayAnimation (Variables|Default|GetSniperScopeWidget) (Variables|/Game/Blueprints/Hud/WBP_SniperScope.WBP_SniperScope_C|GetScopeZoomIn (Variables|Default|GetSniperScopeWidget)) 0.0 1 "Reverse" 1.0 false)
              (Audio|PlaySound2D "/Game/Assets/MilitaryWeapSilver/Sound/SniperRifle/Wavs/SniperRifle_ZoomOut.SniperRifle_ZoomOut" 1.0 1.0 0.0 0 0))))
        (:else)))))

(event EventBeginPlay
  (bind _playerstate (Variables|Default|GetPlayerState))
  (bind _returnvalue (PlayerState|GetPlayerName _playerstate))
  (|CallParentFunction)
  (Networking|SwitchHasAuthority
    (:Authority
      (CallFunction|FSetNameonWidget (PlayerState|GetPlayerName (Game|GetPlayerState 0))))
    (:Remote
      (Variables|Default|GetPlayerState
        (:then
          (CallFunction|FSetNameonWidget _returnvalue)
          (CallFunction|ServerSetPlayerName _returnvalue))
        (:else)))))

(fn ConstructionScript)

(fn FSetNameonWidget
  (params (Name :type String%20%28by%20ref%29))
  (bind _overheadwidget (Variables|Default|GetOverheadWidget)
    (:then
      (Utilities|IsValid (UserInterface|GetUserWidgetObject _overheadwidget)
        (:Is%20Valid
          (bind _aswbp_overhead_widget (Utilities|Casting|CastToWBP_OverheadWidget (UserInterface|GetUserWidgetObject _overheadwidget)))
          (Class|OverheadWidget|ShowPlayerName _aswbp_overhead_widget Name))))
    (:else)))